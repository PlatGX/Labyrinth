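; BP_Target is a target in the Labyrinth laser system that shows its activation state by changing the material on its static mesh.
; It caches the mesh's original material at BeginPlay.
; Activate and deactivate events from its AC_Handler component swap the first material slot between a color-change material and that cached default.
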(event ActivateHandler(AC_Handler)
  (params (Instigator :type AC%20Handler%20Object%20Reference))
  (Rendering|Material|SetMaterial (Variables|Default|GetStaticMesh) 0 (Variables|Default|GetMI_ColorChange)))

(event DeactivateHandler(AC_Handler)
  (params (Instigator :type AC%20Handler%20Object%20Reference))
  (Rendering|Material|SetMaterial (Variables|Default|GetStaticMesh) 0 (Variables|Default|GetMI_DefaultMaterial)))

(event EventBeginPlay
  (Variables|Default|SetMI_DefaultMaterial (Rendering|Material|GetMaterial (Variables|Default|GetStaticMesh) 0)))

(fn ConstructionScript)