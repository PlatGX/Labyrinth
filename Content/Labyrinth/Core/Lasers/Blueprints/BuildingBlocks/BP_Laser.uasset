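; BP_Laser is a laser beam actor that traces forward each tick and stretches its mesh to the blocking hit.
; It sends start, update and stop messages to hit actors' AC_Handler components by diffing this frame's handler set against the last.
; A recursive walk through previous lasers skips handlers already on the beam's path, preventing loops.
; Color changes tint a dynamic material and notify hit handlers; stopping notifies them, then destroys the laser.
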(event EventBeginPlay
  (bind _returnvalue (Rendering|Material|CreateDynamicMaterialInstance "/Game/Labyrinth/Core/Lasers/Materials/MI_Laser.MI_Laser" "None" "None" :!class /Script/Engine.KismetMaterialLibrary))
  (Variables|Default|SetMaterialInstance _returnvalue)
  (Rendering|Material|SetMaterial (Variables|Default|GetStaticMesh) 0 (Variables|Default|GetMaterialInstance))
  (CallFunction|ChangeLaserColor (Variables|Exposed|GetColorOverride)))

(event EventTick
  (params (DeltaSeconds :type Float%20%28single-precision%29))
  (bind _returnvalue (Transformation|GetActorLocation))
  (bind (_outhits _returnvalue_2) (Collision|MultiLineTraceByChannel _returnvalue (+ _returnvalue (* (Transformation|GetActorForwardVector) (Variables|Exposed|GetRange))) "TraceTypeQuery3" false (Variables|Exposed|GetActorsToIgnore) "None"))
  (if _returnvalue_2
    (for _array_element _outhits
      (Utilities|FlowControl|Sequence
        (:then_0
          (if (.bBlockingHit (Collision|BreakHitResult _array_element))
            (CallFunction|UpdateLength (.Distance (Collision|BreakHitResult _array_element)))))
        (:then_1
          (CallFunction|HandleHitActors _array_element))))
    (bind _result (Utilities|Set|Difference (Variables|Default|GetPreviouslyHitHandlers) (Variables|Default|GetCurrentHitHandlers)))
    (bind _result_2 (Utilities|Set|ToArray _result))
    (for _array_element_2 _result_2
      (Class|BPILaser|LaserStopHitting(Message) _array_element_2 self)
      (Utilities|Map|Remove (Variables|Default|GetHittingHandlers) _array_element_2))
    (Variables|Default|SetPreviouslyHitHandlers (Variables|Default|GetCurrentHitHandlers))
    (Utilities|Set|Clear (Variables|Default|GetCurrentHitHandlers))
    (else
      (CallFunction|UpdateLength (Variables|Exposed|GetRange)))))

(event EventLaserStopHitting
  (params (Input :type BP%20Laser%20Object%20Reference))
  (Utilities|FlowControl|Sequence
    (:then_0
      (bind _result (Utilities|Set|ToArray (Variables|Default|GetPreviouslyHitHandlers)))
      (for _array_element _result
        (Class|BPILaser|LaserStopHitting(Message) _array_element self)))
    (:then_1
      (Actor|DestroyActor))))

(fn ConstructionScript)

(fn ChangeLaserColor
  (params (Value :type Linear%20Color%20Structure))
  (Variables|Exposed|SetColorOverride Value)
  (Rendering|Material|SetVectorParameterValue (Variables|Default|GetMaterialInstance) "Color" Value :!class /Script/Engine.MaterialInstanceDynamic)
  (bind _result (Utilities|Set|ToArray (Variables|Default|GetPreviouslyHitHandlers)))
  (for _array_element _result
    (Default|IntermediateChange _array_element self)))

(fn UpdateLength
  (params (InputPin :type Float%20%28single-precision%29))
  (if (not (Math|Float|NearlyEqual(Float) InputPin (Variables|Default|GetPreviousLength) 2.0))
    (bind _output_get (Variables|Default|SetPreviousLength InputPin))
    (Transformation|SetWorldScale3D (Variables|Default|GetStaticMesh) (Math|Vector|MakeVector 0.1 0.1 (/ _output_get 1e+02)))))

(fn HandleHitActors
  (params (InputPin :type Hit%20Result%20Structure))
  (bind _hitactor (Collision|BreakHitResult InputPin))
  (bind _returnvalue (Actor|GetComponentbyClass _hitactor "/Game/Labyrinth/Core/Lasers/Blueprints/BuildingBlocks/AC_Handler.AC_Handler_C"))
  (Utilities|IsValid _returnvalue
    (:Is%20Valid
      (LocalVariables|SetlHandler _returnvalue)
      (if (CallFunction|IsNotonPath (LocalVariables|GetlHandler))
        (Utilities|Map|Add (Variables|Default|GetHittingHandlers) (LocalVariables|GetlHandler) InputPin)
        (if (Utilities|Set|Contains (Variables|Default|GetPreviouslyHitHandlers) (LocalVariables|GetlHandler))
          (Default|LaserUpdateHitting (LocalVariables|GetlHandler) self InputPin)
          (else
            (Class|BPILaser|LaserStartHitting(Message) (LocalVariables|GetlHandler) self InputPin)))
        (Utilities|Set|Add (Variables|Default|GetCurrentHitHandlers) (LocalVariables|GetlHandler))))))

(fn IsNotonPath
  (params (InputHandler :type AC%20Handler%20Object%20Reference))
  (if (Utilities|Array|IsNotEmpty (Variables|Exposed|GetPreviousLasers))
    (for _array_element (Variables|Exposed|GetPreviousLasers)
      (bind _output_get (LocalVariables|SetlCurrentLaser _array_element))
      (if (== (Variables|BP_Laser_C|GetOwningHandler _output_get) InputHandler)
        (return false)
        (elif (not (CallFunction|IsNotonPath (LocalVariables|GetlCurrentLaser) InputHandler))
          (return false))))
    (return true)
    (else
      (return true))))

(fn GetHitbyHandler
  (params (Key :type AC%20Handler%20Object%20Reference%20%28by%20ref%29))
  (bind _hittinghandlers (Variables|Default|GetHittingHandlers))
  (bind (_value _returnvalue) (Utilities|Map|Find _hittinghandlers Key))
  (return _value _returnvalue))