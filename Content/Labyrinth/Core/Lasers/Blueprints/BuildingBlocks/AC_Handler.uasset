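; Actor component that acts as the laser hub for a labyrinth actor, relaying laser hit events to the owner's other BPI_Laser components.
; On BeginPlay it gathers those components, sets the owner's static meshes to block or overlap GameTraceChannel1, and, if InvertSystem is set, calls LaserStopHitting on each emitter.
; Start and stop hits always update the LasersInQueue list, but are forwarded only while the handler is not locked.
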(event EventBeginPlay
  (Utilities|FlowControl|Sequence
    (:then_0
      (bind _output_get (Variables|Default|SetLinkedComponents (Class|Actor|GetComponentsbyInterface (Components|GetOwner) "/Game/Labyrinth/Core/Lasers/Blueprints/BuildingBlocks/BPI_Laser.BPI_Laser_C")))
      (Utilities|Array|RemoveItem _output_get self)
      (for _array_element (Actor|GetComponentsByClass (Components|GetOwner) "/Script/Engine.StaticMeshComponent")
        (Collision|SetCollisionResponsetoChannel _array_element "ECC_GameTraceChannel1" (select (Variables|Conditions|GetIsBlocking) "ECR_Block" "ECR_Overlap"))))
    (:then_1
      (if (Variables|Conditions|GetInvertSystem)
        (for _array_element_2 (Actor|GetComponentsByClass (Components|GetOwner) "/Game/Labyrinth/Core/Lasers/Blueprints/BuildingBlocks/SC_Emitter.SC_Emitter_C")
          ;[0.15 0 0 0.5] ???
          (Default|LaserStopHitting _array_element_2) ; This should be correct.
        )))))

(event EventLaserStartHitting
  (params (Input :type BP%20Laser%20Object%20Reference) (HitInfo :type Hit%20Result%20Structure))
  (CallFunction|LaserAdded Input)
  (Utilities|IsNotLocked
    (:NotLocked
      (bind _array_element (Utilities|ForEachComponent)
        (:LoopBody
          (Class|BPILaser|LaserStartHitting(Message) _array_element Input HitInfo))))))

(event EventLaserStopHitting
  (params (Input :type BP%20Laser%20Object%20Reference))
  (CallFunction|LaserRemoved Input)
  (Utilities|IsNotLocked
    (:NotLocked
      (bind _array_element (Utilities|ForEachComponent)
        (:LoopBody
          (Class|BPILaser|LaserStopHitting(Message) _array_element Input))))))

(fn LaserAdded
  (params (NewItem :type BP%20Laser%20Object%20Reference%20%28by%20ref%29))
  (Utilities|Array|AddUnique (Variables|Default|GetLasersInQueue) NewItem))

(fn LaserRemoved
  (params (NewItem :type BP%20Laser%20Object%20Reference%20%28by%20ref%29))
  (Utilities|Array|RemoveItem (Variables|Default|GetLasersInQueue) NewItem))