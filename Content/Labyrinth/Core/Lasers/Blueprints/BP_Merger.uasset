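; BP_Merger is a laser merger actor in the Labyrinth game, with an emitter mesh that can be rotated in quarter turns.
; Its box collision sets BP_ThirdPersonCharacter's OverlappedObject flag on enter and clears it on exit, storing itself as MergerRef both times.
; The RotateEmitter event steps the emitter's relative yaw by -90 degrees; its caller lies outside this Blueprint.
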(event OnComponentBeginOverlap(BoxCollision)
  (params (OverlappedComponent :type Primitive%20Component%20Object%20Reference) (OtherActor :type Actor%20Object%20Reference) (OtherComp :type Primitive%20Component%20Object%20Reference) (OtherBodyIndex :type Integer) (bFromSweep :type Boolean) (SweepResult :type Hit%20Result%20Structure%20%28by%20ref%29))
  (bind _asbp_third_person_character (Utilities|Casting|CastToBP_ThirdPersonCharacter OtherActor))
  (Variables|/Game/ThirdPerson/Blueprints/BP_ThirdPersonCharacter.BP_ThirdPersonCharacter_C|SetOverlappedObject _asbp_third_person_character true)
  (Variables|/Game/ThirdPerson/Blueprints/BP_ThirdPersonCharacter.BP_ThirdPersonCharacter_C|SetMergerRef _asbp_third_person_character self))

(event OnComponentEndOverlap(BoxCollision)
  (params (OverlappedComponent :type Primitive%20Component%20Object%20Reference) (OtherActor :type Actor%20Object%20Reference) (OtherComp :type Primitive%20Component%20Object%20Reference) (OtherBodyIndex :type Integer))
  (bind _asbp_third_person_character (Utilities|Casting|CastToBP_ThirdPersonCharacter OtherActor))
  (Variables|/Game/ThirdPerson/Blueprints/BP_ThirdPersonCharacter.BP_ThirdPersonCharacter_C|SetOverlappedObject _asbp_third_person_character false)
  (Variables|/Game/ThirdPerson/Blueprints/BP_ThirdPersonCharacter.BP_ThirdPersonCharacter_C|SetMergerRef _asbp_third_person_character self))

(event Custom|RotateEmitter
  (Variables|Default|SetCurrentRotation (Variables|/Script/Engine.SceneComponent|GetRelativeRotation (Variables|Default|GetEmitterMesh)))
  (Transformation|SetRelativeRotation (Variables|Default|GetEmitterMesh) (Math|Rotator|MakeRotator (.roll (Variables|Default|GetCurrentRotation)) (.pitch (Variables|Default|GetCurrentRotation)) (+ (.yaw (Variables|Default|GetCurrentRotation)) -9e+01)) false false))

(fn ConstructionScript)