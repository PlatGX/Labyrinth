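; Actor component that makes its owner start the game hidden and without collision, apparently for later reveal by a Coperfield system.
; On BeginPlay it hides the owning actor and sets every static mesh component to the NoCollision profile.
; Physics-simulating meshes are tagged "MagicPhysic" before simulation is switched off, so it can be restored once visible again.
; It then sets a Ready flag.
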(event EventBeginPlay
  (bind _returnvalue (Components|GetOwner))
  ;[1 1 1] Hide the actor and remove collision during the begin play
  (Utilities|Array|Clear (Variables|Default|GetPhysicsSM))
  (Rendering|SetActorHiddenInGame _returnvalue true)
  (for _array_element (Actor|GetComponentsByClass _returnvalue "/Script/Engine.StaticMeshComponent")
    (if (Physics|IsSimulatingPhysics _array_element "None")
      ;;[1 1 1] Save which Static Mesh Comp is simulating physic to activate it again from Coperfield after becoming visible again
      (Utilities|Array|Add (Variables|/Script/Engine.ActorComponent|GetComponentTags _array_element) "MagicPhysic")
      (Physics|SetSimulatePhysics _array_element false))
    (Collision|SetCollisionProfileName _array_element "NoCollision" true :!class /Script/Engine.PrimitiveComponent))
  (Variables|Default|SetReady true))